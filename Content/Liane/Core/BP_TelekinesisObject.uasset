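; Physics object for a telekinesis mechanic that can be outlined, grabbed, pulled, levitated and thrown.
; Grabbing toggles gravity; pulling uses a negative radial force, levitation lerps toward a destination with random spin, and throwing applies an impulse.
; An overlap field collects mini telekinesis objects, disables their gravity, damps them and pulls them toward the actor each tick until they leave.
; Selection outlines use custom depth on its own and attached actors' meshes.
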(event OnComponentBeginOverlap(AttractionField)
  (params (OverlappedComponent :type Primitive%20Component%20Object%20Reference) (OtherActor :type Actor%20Object%20Reference) (OtherComp :type Primitive%20Component%20Object%20Reference) (OtherBodyIndex :type Integer) (bFromSweep :type Boolean) (SweepResult :type Hit%20Result%20Structure%20%28by%20ref%29))
  ;[1 1 1] Collision Handling
  (bind _asbp_mini_telekinesis_object (Utilities|Casting|CastToBP_MiniTelekinesisObject OtherActor))
  (CallFunction|AddMiniTKObjects _asbp_mini_telekinesis_object))

(event OnComponentEndOverlap(AttractionField)
  (params (OverlappedComponent :type Primitive%20Component%20Object%20Reference) (OtherActor :type Actor%20Object%20Reference) (OtherComp :type Primitive%20Component%20Object%20Reference) (OtherBodyIndex :type Integer))
  ;[1 1 1] Collision Handling
  (bind _asbp_mini_telekinesis_object (Utilities|Casting|CastToBP_MiniTelekinesisObject OtherActor))
  (CallFunction|RemoveMiniTKObjects _asbp_mini_telekinesis_object))

(event EventBeginPlay
  (bind _mesh (Variables|Default|GetMesh))
  (Physics|SetSimulatePhysics _mesh true)
  (Physics|SetEnableGravity _mesh true)
  (CallFunction|PrepareOutline))

(event EventTick
  (params (DeltaSeconds :type Float%20%28single-precision%29))
  (CallFunction|AttractMiniTKObjects))

(fn ConstructionScript)

(fn GetThrowableMeshLocation
  (return (Transformation|GetWorldLocation (Variables|Default|GetMesh))))

(fn GetAllChildrenMeshes
  (bind _localactors (LocalVariables|GetLocalActors))
  (Utilities|Array|Add _localactors self)
  (Utilities|Array|AppendArray _localactors (Actor|GetAttachedActors false))
  (for _array_element _localactors
    (Utilities|Array|AppendArray (LocalVariables|GetAllMeshes) (Actor|GetComponentsByClass _array_element "/Script/Engine.MeshComponent")))
  (return (LocalVariables|GetAllMeshes)))

(fn PrepareOutline
  (bind _meshes (CallFunction|GetAllChildrenMeshes))
  (for _array_element _meshes
    (bind _asmesh_component (Utilities|Casting|CastToMeshComponent _array_element))
    (Rendering|SetCustomDepthStencilValue _asmesh_component 1)))

(fn SetSelectionOutlineVisible
  (params (IsOutlineVisible :type Boolean))
  (bind _meshes (CallFunction|GetAllChildrenMeshes))
  ;[1 1 1] Enable outline on mesh components
  (for _array_element _meshes
    (bind _asmesh_component (Utilities|Casting|CastToMeshComponent _array_element))
    (Rendering|SetRenderCustomDepth _asmesh_component IsOutlineVisible)))

(fn SetasGrabbed
  (params (IsGrabbed :type Boolean))
  (Physics|SetEnableGravity (Variables|Default|GetMesh) (not IsGrabbed)))

(fn Attract
  (params (Destination :type Vector))
  (Physics|AddRadialForce (Variables|Default|GetMesh) Destination 1e+05 -3e+04 "RIF_Constant" true))

(fn Levitate
  (params (Destination :type Vector))
  (bind _mesh (Variables|Default|GetMesh))
  (Transformation|SetWorldLocation _mesh (Math|Vector|Lerp(Vector) (Transformation|GetWorldLocation (Variables|Default|GetMesh)) Destination (/ (* (Utilities|Time|GetWorldDeltaSeconds) 0.5) 0.1)) true false)
  (Physics|SetPhysicsLinearVelocity _mesh "0, 0, 0" false "None")
  (Class|PrimitiveComponent|AddAngularImpulseinDegrees _mesh (Math|Vector|MakeVector (Math|Random|RandomFloatinRange -1e+01 1e+01) (Math|Random|RandomFloatinRange -1e+01 1e+01) (Math|Random|RandomFloatinRange -1e+01 1e+01)) "None" true))

(fn Throw
  (params (Orientation :type Vector))
  (Physics|AddImpulse (Variables|Default|GetMesh) (* Orientation 1e+04) "None" true))

(fn AttractMiniTKObjects
  (for _array_element (Variables|Default|GetMini%20TK%20Objects)
    (Default|AttractForce _array_element (* (Math|Vector|GetUnitDirection(Vector) (Transformation|GetActorLocation _array_element) (Transformation|GetActorLocation)) (Variables|Default|GetMiniTKObjectAttractForce)))))

(fn AddMiniTKObjects
  (params (Mini%20TKObject :type BP%20Mini%20Telekinesis%20Object%20Object%20Reference%20%28by%20ref%29))
  (bind _staticmesh (Variables|/Game/Liane/Core/BP_MiniTelekinesisObject.BP_MiniTelekinesisObject_C|GetStaticMesh Mini%20TKObject))
  (Utilities|Array|Add (Variables|Default|GetMini%20TK%20Objects) Mini%20TKObject)
  (Physics|SetEnableGravity _staticmesh false)
  (Class|PrimitiveComponent|SetLinearDamping _staticmesh (Variables|Default|GetIn%20Damping)))

(fn RemoveMiniTKObjects
  (params (MiniTKObject :type BP%20Mini%20Telekinesis%20Object%20Object%20Reference%20%28by%20ref%29))
  (bind _staticmesh (Variables|/Game/Liane/Core/BP_MiniTelekinesisObject.BP_MiniTelekinesisObject_C|GetStaticMesh MiniTKObject))
  (Utilities|Array|RemoveItem (Variables|Default|GetMini%20TK%20Objects) MiniTKObject)
  (Physics|SetEnableGravity _staticmesh true)
  (Class|PrimitiveComponent|SetLinearDamping _staticmesh 0.0))